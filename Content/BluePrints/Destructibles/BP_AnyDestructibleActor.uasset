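; A generic destructible actor that is destroyed when it receives damage, with its look and effects defined by a DestructibleType reference.
; The construction script applies that type's mesh to the StaticMesh component if the reference is valid.
; The DealDamage interface event plays the type's death sound and spawns its particle effect at the mesh location, then immediately destroys the actor, with no health tracking.
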(event `self.DealDamage`
  (params (DamageAmount :type "Float (double-precision)"))
  (bind _destructibletype (`self.DestructibleType`))
  (bind _returnvalue (`SceneComponent.K2_GetComponentLocation` (`self.StaticMesh`)))
  ;[1 1 1] INTERFACE function. Play a sound, spawn a particle effect and destroy this actor
  (`GameplayStatics.PlaySoundAtLocation` (`/Game/DataAssets/DestructibleDataAsset.DeathSoundEffect` _destructibletype) _returnvalue (struct) 1.0 1.0 0.0 null null null null)
  (`GameplayStatics.SpawnEmitterAtLocation` (`/Game/DataAssets/DestructibleDataAsset.ParticleEffectOnDestruct` _destructibletype) _returnvalue)
  (`self.K2_DestroyActor`))

(fn `UserConstructionScript`
  ;[1 1 1] Set the mesh
  (bind _destructibletype (`self.DestructibleType`)
    (:`then`
      (`StaticMeshComponent.SetStaticMesh` (`self.StaticMesh`) (`/Game/DataAssets/DestructibleDataAsset.Mesh` _destructibletype)))
    (:`else`)))