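; Game manager Blueprint that handles player respawning and the respawn screen.
; BeginPlay creates the respawn widget hidden.
; RespawnPlayer shows it, teleports the player above the first PlayerStart, plays a sound and restores health and its widget, toggling the freeze flag within the same call.
; Tick hides the widget through a Delay while PlayerRespawned is true, a flag this Blueprint never clears.
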(event `self.ReceiveBeginPlay`
  ;[1 1 1] Create the respawn widget, get a reference to it and make it hidden at the start
  (bind _returnvalue (`|CreateWidget` "/Game/Widgets/Game_Notification_Widgets/WB_Respawn.WB_Respawn_C"))
  (bind _output_get (set `self.RefToRespawnWidget` _returnvalue))
  (`UserWidget.AddToViewport` _output_get 0)
  (set `Widget.Visibility` "Hidden" _output_get))

(event `self.ReceiveTick`
  (params (DeltaSeconds :type "Float (single-precision)"))
  ;[1 1 1] IF player respawned, then have delay before hiding the respawn widget
  (if (`self.playerRespawned`)
    (`KismetSystemLibrary.Delay` 2.0)
    (set `Widget.Visibility` "Hidden" (`self.RefToRespawnWidget`))))

(fn `RespawnPlayer`
  (bind _returnvalue (`GameplayStatics.GetPlayerCharacter` 0))
  ;[1 1 1] Make respawn widget visible
  (set `Widget.Visibility` "Visible" (`self.RefToRespawnWidget`))
  ;[1 1 1] Prevent player movement
  (bind _asbp_third_person_character (cast `` _returnvalue))
  (set `/Game/BluePrints/GameManager/BP_GameManager.freezePlayer` true _asbp_third_person_character)
  ;[1 1 1] Find player start location and set player locatiion to this
  (bind _outactors (`GameplayStatics.GetAllActorsOfClass` "/Script/Engine.PlayerStart"))
  (bind (_returnvalue_x _returnvalue_y _returnvalue_z) (`KismetMathLibrary.BreakVector` (`self.K2_GetActorLocation` (`|GetArrayItem` _outactors))))
  (bind _returnvalue_2 (+ _returnvalue_z 1000.0))
  (`self.K2_SetActorLocation` _returnvalue (`KismetMathLibrary.MakeVector` _returnvalue_x _returnvalue_y _returnvalue_2) false false)
  ;[1 1 1] Play respawn sound, set player health to 100, reset health in health widget and un-freeze player movement
  (`GameplayStatics.PlaySoundAtLocation` "/Game/Sounds/Respawn_Sound.Respawn_Sound" (`KismetMathLibrary.MakeVector` _returnvalue_x _returnvalue_y _returnvalue_2) (struct) 1.0 1.0 0.0 null null null null)
  (bind _output_get (set `/Game/BluePrints/GameManager/BP_GameManager.playerHealth` 100.0 _asbp_third_person_character))
  (set `/Game/Widgets/PlayerWidgets/WB_PlayerHealth.playerHealth` _output_get (`/Game/BluePrints/GameManager/BP_GameManager.RefToHealthWidget` _asbp_third_person_character))
  (set `/Game/BluePrints/GameManager/BP_GameManager.freezePlayer` false _asbp_third_person_character)
  (set `self.playerRespawned` true))

(fn `UserConstructionScript`)