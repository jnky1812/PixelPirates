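; Coin pickup actor that takes its mesh, base money and base XP from an ItemType data asset.
; On BeginPlay it caches the player and fixes its coin value from base money plus a random bonus, scaled by player level.
; An overlap passing a cast adds that value through the first BP_MoneyManager found, grants XP scaled by current level, plays a sound and destroys the actor.
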(event `self.ReceiveBeginPlay`
  (`KismetSystemLibrary.PrintString` "Coin Spawned")
  ;[1 1 1] Set player reference
  (bind _asbp_third_person_character (cast `` (`GameplayStatics.GetPlayerCharacter` 0)))
  (set `self.RefToPlayer` _asbp_third_person_character)
  ;[1 1 1] Set coin's value at start
  (`self.DetermineCoinValue`))

(event `self.StaticMesh.OnComponentBeginOverlap`
  (params (OverlappedComponent :type "PrimitiveComponent Object Reference") (OtherActor :type "Actor Object Reference") (OtherComp :type "PrimitiveComponent Object Reference") (OtherBodyIndex :type Integer) (bFromSweep :type Boolean) (SweepResult :type "HitResult Structure (by ref)"))
  (cast `` OtherActor)
  (`self.AddMoneyToPlayer`))

(fn `AddMoneyToPlayer`
  ;[1 1 1] Add money, add XP, play sound and destroy this actor
  (bind _outactors (`GameplayStatics.GetAllActorsOfClass` "/Game/BluePrints/Money/BP_MoneyManager.BP_MoneyManager_C"))
  (`/Game/BluePrints/Money/BP_MoneyManager.Add Money` (`|GetArrayItem` _outactors) (`self.coinValue`))
  (bind _asbp_third_person_character (cast `` (`GameplayStatics.GetPlayerCharacter` 0)))
  (bind _returnvalue (`self.DetermineXP`))
  (`self.AddXP` _asbp_third_person_character _returnvalue)
  (`GameplayStatics.PlaySound2D` "/Game/Sounds/Money_Sound.Money_Sound" 1.0 1.0 0.0 null null)
  (`self.K2_DestroyActor`))

(fn `DetermineCoinValue`
  ;[1 1 1] Algo for setting coin value. Based on player level and some randomisation
  (set `self.coinValue` (`KismetMathLibrary.FTrunc` (* (+ (`/Game/DataAssets/MoneyDataAsset.moneyOnPickup` (`self.itemType`)) (`KismetMathLibrary.RandomIntegerInRange` 0 10)) (/ (`KismetMathLibrary.Conv_IntToDouble` (`/Game/BluePrints/Money/BP_MoneyDataAssetActor.playerLevel` (`self.RefToPlayer`))) 2.0))))
  (return))

(fn `DetermineXP`
  (returns (ReturnValue :type Integer))
  (return (`KismetMathLibrary.FTrunc` (* (`/Game/DataAssets/MoneyDataAsset.XPonPickup` (`self.itemType`)) (/ (`KismetMathLibrary.Conv_IntToDouble` (`/Game/BluePrints/Money/BP_MoneyDataAssetActor.playerLevel` (`self.RefToPlayer`))) 2.0)))))

(fn `UserConstructionScript`
  ;[1 1 1] Sets the mesh
  (bind _itemtype (`self.itemType`)
    (:`then`
      (`StaticMeshComponent.SetStaticMesh` (`self.StaticMesh`) (`/Game/DataAssets/MoneyDataAsset.Mesh` _itemtype)))
    (:`else`)))