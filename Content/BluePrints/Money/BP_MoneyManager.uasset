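; BP_MoneyManager is an actor that tracks the player's money and shows it on screen.
; On BeginPlay it gets a WB_PlayerMoney widget from its MoneyWidget component, pushes the current PlayerMoney value into it and adds it to the viewport.
; AddMoney increases PlayerMoney by the given amount and refreshes the widget through the cached reference.
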(event `self.ReceiveBeginPlay`
  ;[1 1 1] Sets reference to widget, updates player money in widget and makes it visible
  (bind _aswb_player_money (cast `/Game/Widgets/MoneyWidget/WB_PlayerMoney` (`WidgetComponent.GetUserWidgetObject` (`self.MoneyWidget`))))
  (bind _output_get (set `self.RefToPlayerMoney` _aswb_player_money))
  (`/Game/Widgets/MoneyWidget/WB_PlayerMoney.UpdateMoney` _output_get (`self.playerMoney`))
  (`UserWidget.AddToViewport` (`self.RefToPlayerMoney`) 0))

(fn `Add Money`
  (params (AmountToAdd :type Integer))
  ;[1 1 1] Adds money then updates widget
  (bind _output_get (set `self.playerMoney` (+ AmountToAdd (`self.playerMoney`))))
  (`/Game/Widgets/MoneyWidget/WB_PlayerMoney.UpdateMoney` (`self.RefToPlayerMoney`) _output_get))

(fn `UserConstructionScript`)