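; Harvestable tree actor that takes its mesh and wood and coconut yields from a FoilageType data asset.
; It starts at one-third scale and yield, then grows and gains resources at timed maturity levels driven by Tick.
; DealDamage plays chop feedback with a brief material flash, and every MaxChopCount hits spawns available wood and coconut collectibles.
; Tick destroys the tree once its drop count reaches WoodPerTree.
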(event `self.ReceiveBeginPlay`
  (bind (_returnvalue_location _returnvalue_rotation _returnvalue_scale) (`KismetMathLibrary.BreakTransform` (`self.GetTransform`)))
  ;[1 1 1] Initialise tree scale for a level-1 tree
  (`self.K2_SetActorTransform` (`KismetMathLibrary.MakeTransform` _returnvalue_location _returnvalue_rotation (* _returnvalue_scale 0.33)))
  ;[1 1 1] Set coconuts available
  (set `self.currentCoconutsAvailabeToHarvest` (`KismetMathLibrary.Round` (* (`KismetMathLibrary.Conv_IntToDouble` (`/Game/DataAssets/FoilageDataAsset.coconutsPerTree` (`self.foilageType`))) 0.33)))
  ;[1 1 1] Set wood available
  (set `self.currentWoodAvailableToHarvest` (`KismetMathLibrary.Round` (* (`KismetMathLibrary.Conv_IntToDouble` (`/Game/DataAssets/FoilageDataAsset.woodPerTree` (`self.foilageType`))) 0.33)))
  ;[1 1 1] Get reference to material
  (set `self.startingMaterial` (`PrimitiveComponent.GetMaterial` (`self.StaticMesh`) 1)))

(event `self.ReceiveTick`
  (params (DeltaSeconds :type "Float (single-precision)"))
  (`|ExecutionSequence`
    (:`then_0`
      ;[1 1 1] Handles tree maturing
      (if (< (`self.currentTreeMaturity`) (`self.maxTreeMaturity`))
        (`self.IncreaseTreeMaturityEachTick` DeltaSeconds)
        (bind _treecanmature (`self.CanTreeMatureToNextLevel`))
        (if _treecanmature
          (`self.MatureTreeToNextLevel`))))
    (:`then_1`
      ;[1 1 1] Destroy tree if all wood is gone
      (if (>= (`self.timesWoodDropped`) (`/Game/DataAssets/FoilageDataAsset.woodPerTree` (`self.foilageType`)))
        (`self.K2_DestroyActor`)))
    (:`then_2`
      ;[1 1 1] Reset material after a delay
      (if (`self.materialChangedOnHit`)
        (`KismetSystemLibrary.Delay` 0.2)
        (`self.Reset Material`)))))

(event `self.DealDamage`
  (params (DamageAmount :type "Float (double-precision)"))
  ;[1 1 1] Try to harvest wood +/- coconuts
  (`self.CanHarvestWoodAndCoconuts`))

(fn `CanHarvestWoodAndCoconuts`
  (bind _chopcount (`self.chopCount`))
  (bind _returnvalue (+ (`self.K2_GetActorLocation`) (0.0 100.0 0.0)))
  (bind _returnvalue_2 (+ (`self.K2_GetActorLocation`) (50.0 -150.0 0.0)))
  (`GameplayStatics.PlaySound2D` "/Game/Sounds/ChopWood_Sound.ChopWood_Sound" 1.0 1.0 0.0 null null)
  ;[1 1 1] Add to chop count. See if can spawn wood +/- coconuts
  (if (< _chopcount (`self.maxChopCount`))
    (bind _result (`/Engine/EditorBlueprintResources/StandardMacros.IncrementInt` _chopcount)
      (:`  `
        (set `self.chopCount` _result)
        (`self.ColourFlash`)))
    (else
      (`self.ColourFlash`)))
  (if (>= (`self.chopCount`) (`self.maxChopCount`))
    (set `self.chopCount` 0)
    (bind _result_2 (`/Engine/EditorBlueprintResources/StandardMacros.IncrementInt` (`self.timesWoodDropped`))
      (:`  `
        (set `self.timesWoodDropped` _result_2)
        (if (> (`self.currentWoodAvailableToHarvest`) 0)
          (`|SpawnActorFromClass` "/Game/BluePrints/Collectibles/BP_CollectibleDataAssetActor.BP_CollectibleDataAssetActor_C" (`KismetMathLibrary.MakeTransform` _returnvalue (struct) (0.02 0.02 0.02)) "Undefined" "MultiplyWithRoot" null "/Game/DataAssets/Foilage/Wood.Wood" null)
          (`GameplayStatics.PlaySoundAtLocation` "/Game/Sounds/LootDrop_Sound.LootDrop_Sound" _returnvalue (struct) 1.0 1.0 0.0 null null null null)
          (bind _result_3 (`/Engine/EditorBlueprintResources/StandardMacros.DecrementInt` (`self.currentWoodAvailableToHarvest`))
            (:`  `
              (set `self.currentWoodAvailableToHarvest` _result_3))))
        (if (> (`self.currentCoconutsAvailabeToHarvest`) 0)
          (`|SpawnActorFromClass` "/Game/BluePrints/Collectibles/BP_CollectibleDataAssetActor.BP_CollectibleDataAssetActor_C" (`KismetMathLibrary.MakeTransform` _returnvalue_2) "Undefined" "MultiplyWithRoot" null "/Game/DataAssets/Consumables/Coconut.Coconut" null)
          (`GameplayStatics.PlaySoundAtLocation` "/Game/Sounds/LootDrop_Sound.LootDrop_Sound" _returnvalue_2 (struct) 1.0 1.0 0.0 null null null null)
          (bind _result_4 (`/Engine/EditorBlueprintResources/StandardMacros.DecrementInt` (`self.currentCoconutsAvailabeToHarvest`))
            (:`  `
              (set `self.currentCoconutsAvailabeToHarvest` _result_4))))))))

(fn `CanTreeMatureToNextLevel`
  (returns (TreeCanMature :type Boolean))
  ;[1 1 1] Determines if tree can level up maturity. If so, tree flashes a colour, levels up and resets current time
  (if (>= (`self.currentTime`) (`self.maturityTime`))
    (if (< (`self.currentTreeMaturity`) (`self.maxTreeMaturity`))
      (set `self.currentTime` 0.0)
      (bind _result (`/Engine/EditorBlueprintResources/StandardMacros.IncrementInt` (`self.currentTreeMaturity`))
        (:`  `
          (set `self.currentTreeMaturity` _result)
          (return true)))
      (else
        (return false)))
    (else
      (return false))))

(fn `ColourFlash`
  ;[1 1 1] Change material
  (`PrimitiveComponent.SetMaterial` (`self.StaticMesh`) 1 "/Game/Materials/Green_Mat.Green_Mat")
  (set `self.materialChangedOnHit` true))

(fn `IncreaseTreeMaturityEachTick`
  (params (tickTime :type "Float (double-precision)"))
  ;[1 1 1] Increases the current time each tick
  (set `self.currentTime` (+ tickTime (`self.currentTime`))))

(fn `MatureTreeToNextLevel`
  (bind (_returnvalue_location _returnvalue_rotation _returnvalue_scale) (`KismetMathLibrary.BreakTransform` (`self.GetTransform`)))
  ;[1 1 1] Scale up the tree
  (`self.K2_SetActorTransform` (`KismetMathLibrary.MakeTransform` _returnvalue_location _returnvalue_rotation (+ _returnvalue_scale 0.33)))
  ;[1 1 1] Add extra coconuts
  (set `self.currentCoconutsAvailabeToHarvest` (+ (`self.currentCoconutsAvailabeToHarvest`) (`KismetMathLibrary.Round` (* (`KismetMathLibrary.Conv_IntToDouble` (`/Game/DataAssets/FoilageDataAsset.coconutsPerTree` (`self.foilageType`))) 0.33))))
  ;[1 1 1] Add extra wood
  (set `self.currentWoodAvailableToHarvest` (+ (`self.currentWoodAvailableToHarvest`) (`KismetMathLibrary.Round` (* (`KismetMathLibrary.Conv_IntToDouble` (`/Game/DataAssets/FoilageDataAsset.woodPerTree` (`self.foilageType`))) 0.33)))))

(fn `Reset Material`
  ;[1 1 1] Reset material to starting material
  (`PrimitiveComponent.SetMaterial` (`self.StaticMesh`) 1 (`self.startingMaterial`))
  (set `self.materialChangedOnHit` false))

(fn `UserConstructionScript`
  ;[1 1 1] Set the mesh
  (bind _foilagetype (`self.foilageType`)
    (:`then`
      (`StaticMeshComponent.SetStaticMesh` (`self.StaticMesh`) (`/Game/DataAssets/FoilageDataAsset.Mesh` _foilagetype)))
    (:`else`)))