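; Collectible chest Blueprint that opens its lid when the player character overlaps it and closes it when the player leaves.
; Begin and end overlap events call custom open and close events, which play or reverse a single timeline.
; The timeline's float track scales the lid's relative rotation, so the same curve drives both directions of the swing.
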(event `self.ReceiveActorBeginOverlap`
  (params (OtherActor :type "Actor Object Reference"))
  ;[1 1 1] Player overlap events to trigger custom events
  (if (== OtherActor (`GameplayStatics.GetPlayerCharacter` 0))
    (`self.OpenChest`)))

(event `self.ReceiveActorEndOverlap`
  (params (OtherActor :type "Actor Object Reference"))
  ;[1 1 1] Player overlap events to trigger custom events
  (if (== OtherActor (`GameplayStatics.GetPlayerCharacter` 0))
    (`self.CloseChest`)))

(event `OpenChest`
  ;[1 1 1] USe TimeLine to alter the rotation value of X
  (bind (_direction _liposition) (`Timeline|ChestOpen` :!label _label)
    (:`Update`
      (`SceneComponent.K2_SetRelativeRotation` (`self.Lid`) (* (struct :`Roll` -120.0) _liposition) false false))))

(event `CloseChest`
  ;[1 1 1] USe TimeLine to alter the rotation value of X
  (goto _label :!via `Reverse`))

(fn `UserConstructionScript`)