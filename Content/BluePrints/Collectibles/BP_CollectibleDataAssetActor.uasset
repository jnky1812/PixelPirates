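; Collectible pickup actor driven by an ItemType data asset, whose mesh the construction script applies to its StaticMesh.
; The "press E" prompt, overlap and input-polling logic is disconnected, leaving the Tick and overlap events empty.
; PickupItem only clears CanPickupItem and runs an unused actor search, while inventory and XP steps are unwired and AddXP just destroys the actor.
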(event `self.ReceiveBeginPlay`)

(event `self.ReceiveActorBeginOverlap`
  (params (OtherActor :type "Actor Object Reference")))

(event `resetDoOnce`
  ;[1 1 1] Pickup item when "E" pressed
  (`/Engine/EditorBlueprintResources/StandardMacros.DoOnce` false :!via `Reset`
    (:`Completed`
      (`self.PickupItem`))))

(event `self.ReceiveTick`
  (params (DeltaSeconds :type "Float (single-precision)")))

(event `self.StaticMesh.OnComponentBeginOverlap`
  (params (OverlappedComponent :type "PrimitiveComponent Object Reference") (OtherActor :type "Actor Object Reference") (OtherComp :type "PrimitiveComponent Object Reference") (OtherBodyIndex :type Integer) (bFromSweep :type Boolean) (SweepResult :type "HitResult Structure (by ref)")))

(event `self.StaticMesh.OnComponentEndOverlap`
  (params (OverlappedComponent :type "PrimitiveComponent Object Reference") (OtherActor :type "Actor Object Reference") (OtherComp :type "PrimitiveComponent Object Reference") (OtherBodyIndex :type Integer)))

(fn `PickupItem`
  ;[1 1 1] Add item to inventory. Add player XP
  (if (`self.canPickupItem`)
    (set `self.canPickupItem` false)
    (bind _outactors (`GameplayStatics.GetAllActorsOfClass` null))))

(fn `UserConstructionScript`
  (bind _itemtype (`self.ItemType`)
    (:`then`
      (`StaticMeshComponent.SetStaticMesh` (`self.StaticMesh`) (`/Game/DataAssets/ResourceDataAsset.Mesh` _itemtype)))
    (:`else`)))