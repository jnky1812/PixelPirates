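; BP_EnemySpawner is a spawner actor that keeps populating an area with AI enemies.
; On BeginPlay it starts a looping timer that fires SpawnEnemy at the configured interval.
; Each tick counts every actor of the enemy class in the world and, while below the maximum, spawns an enemy pawn at a random point inside its Box bounds.
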(event `Spawn Enemy`
  ;[1 1 1] spawn enemy upto value of Max number of enemies
  (bind _outactors (`GameplayStatics.GetAllActorsOfClass` (`self.EnemyActor`)))
  (if (< (`KismetArrayLibrary.Array_Length` _outactors) (`self.MaxNumber of Enemies`))
    (`AIBlueprintHelperLibrary.SpawnAIFromClass` (`self.Enemy Pawn`) null (`KismetMathLibrary.RandomPointInBoundingBox` (`SceneComponent.K2_GetComponentLocation` (`self.DefaultSceneRoot`)) (`BoxComponent.GetScaledBoxExtent` (`self.Box`))) (struct) false null)))

(event `self.ReceiveBeginPlay`
  ;[1 1 1] Spawn timer
  (`KismetSystemLibrary.K2_SetTimerDelegate` (delegate `Spawn Enemy`) (`self.SpawnTime`) true))

(fn `UserConstructionScript`)