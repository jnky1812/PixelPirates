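; Crab enemy NPC that roams random nearby points and chases the player once PawnSensing spots them, playing an attack animation on arrival.
; DealDamage applies doubled damage to Health, updates the widget health bar and triggers death sound and blood effects at zero.
; Contact damage and health-bar visibility logic is disconnected.
; AddXP destroys the actor and drops meat and shell loot but awards no XP and is never called here.
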(event `self.ReceiveBeginPlay`
  (`self.RoamAround`)
  ;[1 1 1] Reference the health bar widget
  (bind _aswbp_enemy (cast `/Game/BluePrints/NPCs/Crab/WBP_Enemy` (`WidgetComponent.GetUserWidgetObject` (`self.Widget`))))
  (set `self.HealthWidgetRef` _aswbp_enemy))

(event `RoamAround`
  ;[1 1 1] Roam Around AI
  (`|AIMoveTo` self (`NavigationSystemV1.K2_GetRandomReachablePointInRadius` (`self.K2_GetActorLocation`) 500.0 null null) null 120.0
    (:`OnSuccess`
      (`KismetSystemLibrary.Delay` 1.2)
      (`SkeletalMeshComponent.PlayAnimation` (`self.Mesh`) "/Game/Meshes/NPCs/AnimatedCrab/CrabAnimRigCrab_Walk_Anim.CrabAnimRigCrab_Walk_Anim" true)
      (`self.RoamAround`))))

(event `self.PawnSensing.OnSeePawn`
  (params (Pawn :type "Pawn Object Reference"))
  ;[1 1 1] Follow player AI
  (set `self.IsSeeingPlayer` true)
  (`self.FollowPlayer`))

(event `FollowPlayer`
  ;[1 1 1] Follow player AI
  (if (`self.IsSeeingPlayer`)
    (`|AIMoveTo` self (0.0 0.0 0.0) (`GameplayStatics.GetPlayerCharacter` 0)
      (:`OnSuccess`
        (`SkeletalMeshComponent.PlayAnimation` (`self.Mesh`) "/Game/Meshes/NPCs/AnimatedCrab/CrabAnimRigCrab_Attack_Anim.CrabAnimRigCrab_Attack_Anim" true))
      (:`OnFail`
        (set `self.IsSeeingPlayer` false)
        (`self.RoamAround`)))))

(event `self.Sphere.OnComponentBeginOverlap`
  (params (OverlappedComponent :type "PrimitiveComponent Object Reference") (OtherActor :type "Actor Object Reference") (OtherComp :type "PrimitiveComponent Object Reference") (OtherBodyIndex :type Integer) (bFromSweep :type Boolean) (SweepResult :type "HitResult Structure (by ref)"))
  ;[1 1 1] Health visability
)

(event `self.Sphere.OnComponentEndOverlap`
  (params (OverlappedComponent :type "PrimitiveComponent Object Reference") (OtherActor :type "Actor Object Reference") (OtherComp :type "PrimitiveComponent Object Reference") (OtherBodyIndex :type Integer))
  ;[1 1 1] Health visability
)

(event `self.DamageCollision.OnComponentBeginOverlap`
  (params (OverlappedComponent :type "PrimitiveComponent Object Reference") (OtherActor :type "Actor Object Reference") (OtherComp :type "PrimitiveComponent Object Reference") (OtherBodyIndex :type Integer) (bFromSweep :type Boolean) (SweepResult :type "HitResult Structure (by ref)"))
  ;[1 1 1] damage
)

(event `self.DamageCollision.OnComponentEndOverlap`
  (params (OverlappedComponent :type "PrimitiveComponent Object Reference") (OtherActor :type "Actor Object Reference") (OtherComp :type "PrimitiveComponent Object Reference") (OtherBodyIndex :type Integer))
  ;[1 1 1] damage
)

(event `self.DealDamage`
  (params (DamageAmount :type "Float (double-precision)"))
  ;[1 1 1] INTERFACE function that deals damage to the crab
  (bind _output_get (set `self.Health` (- (`self.Health`) (* DamageAmount 2.0))))
  (`/Game/BluePrints/NPCs/Crab/WBP_Enemy.UpdateHealth` (`self.HealthWidgetRef`) _output_get)
  (if (<= (`self.Health`) 0.0)
    (`self.DeathSequence`)))

(fn `DeathSequence`
  (bind _returnvalue (`SceneComponent.K2_GetComponentLocation` (`self.Mesh`)))
  ;[1 1 1] Play sound, spawn particle effect, add XP to player and destroy THIS actor
  (`GameplayStatics.PlaySoundAtLocation` "/Game/Sounds/Splat_Sound.Splat_Sound" _returnvalue (struct) 1.0 1.0 0.0 null null null null)
  (`GameplayStatics.SpawnEmitterAtLocation` "/Game/Realistic_Starter_VFX_Pack_Vol2/Particles/Blood/P_Blood_Splat_Cone.P_Blood_Splat_Cone" _returnvalue))

(fn `LootDrop`
  (bind _returnvalue (`self.GetTransform`))
  (bind _returnvalue_2 (`self.GetTransform`))
  ;[1 1 1] Spawn loot
  (`|SpawnActorFromClass` "/Game/BluePrints/Collectibles/BP_CollectibleDataAssetActor.BP_CollectibleDataAssetActor_C" (`KismetMathLibrary.MakeTransform` (`KismetMathLibrary.MakeVector` (+ (.x (.location _returnvalue_2)) 20.0) (.y (.location _returnvalue_2)) (.z (.location _returnvalue_2))) (.rotation _returnvalue_2) (.scale _returnvalue_2)) "AdjustIfPossibleButAlwaysSpawn" "MultiplyWithRoot" null "/Game/DataAssets/Consumables/DA_CrabMeat.DA_CrabMeat" null)
  (`|SpawnActorFromClass` "/Game/BluePrints/Collectibles/BP_CollectibleDataAssetActor.BP_CollectibleDataAssetActor_C" (`KismetMathLibrary.MakeTransform` (`KismetMathLibrary.MakeVector` (+ (.x (.location _returnvalue)) -20.0) (.y (.location _returnvalue)) (.z (.location _returnvalue))) (.rotation _returnvalue) (.scale _returnvalue)) "AdjustIfPossibleButAlwaysSpawn" "MultiplyWithRoot" null "/Game/DataAssets/Collectibles/DA_CrabShell.DA_CrabShell" null))

(fn `UserConstructionScript`
  (`self.RoamAround`))